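; Tower defense turret that fires BP_Bullet at one enemy at a time and levels up from XP.
; BeginPlay loads the hardcoded "AoE" data table row to set mesh, range and stats.
; Range-sphere overlaps set or clear the target; without one, Tick runs a throttled sphere trace for the closest enemy.
; With a target, Tick fires on a fire-rate delay, scaling damage by level and passing itself as bullet owner.
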(event OnComponentBeginOverlap(Sphere)
  (params (OverlappedComponent :type Primitive%20Component%20Object%20Reference) (OtherActor :type Actor%20Object%20Reference) (OtherComp :type Primitive%20Component%20Object%20Reference) (OtherBodyIndex :type Integer) (bFromSweep :type Boolean) (SweepResult :type Hit%20Result%20Structure%20%28by%20ref%29))
  (Utilities|IsValid (Variables|Default|GetCurrentTarget)
    (:Is%20Not%20Valid
      (bind _asenemy (Utilities|Casting|CastToEnemy OtherActor))
      (Variables|Default|SetCurrentTarget _asenemy))))

(event OnComponentEndOverlap(Sphere)
  (params (OverlappedComponent :type Primitive%20Component%20Object%20Reference) (OtherActor :type Actor%20Object%20Reference) (OtherComp :type Primitive%20Component%20Object%20Reference) (OtherBodyIndex :type Integer))
  (if (== OtherActor (Variables|Default|GetCurrentTarget))
    (Variables|Default|SetCurrentTarget 0)))

(event Custom|MakeTower
  (bind _towerstruct (Variables|Default|GetTowerStruct))
  (bind (_name _damage _range _firerate _mesh) (Utilities|Struct|BreakTowerStruct _towerstruct))
  (Components|StaticMesh|SetStaticMesh (Variables|Default|GetTowerMesh) _mesh)
  (Components|Sphere|SetSphereRadius (Variables|Default|GetSphere) _range true))

(event Custom|BulletInit
  (bind _towerstruct (Variables|Default|GetTowerStruct))
  (bind (_name _damage _range _firerate _mesh _particle) (Utilities|Struct|BreakTowerStruct _towerstruct))
  (Variables|Default|SetReload true)
  (Game|SpawnActorfromClass "/Game/Towers/BP_Bullet.BP_Bullet_C" (Transformation|GetActorTransform) "AlwaysSpawn" 0 (Variables|Default|GetCurrentTarget) (* (+ (/ (Math|Conversions|ToFloat(Integer) (Variables|Default|GetCurrentLevel)) 1e+01) 1.0) _damage) self 0)
  (Utilities|FlowControl|Delay _firerate)
  (Variables|Default|SetReload false))

(event Custom|FindTarget
  (bind _returnvalue (Transformation|GetActorLocation))
  (Variables|Default|SetCheckForTarget true)
  (bind (_outhits _returnvalue_2) (Collision|MultiSphereTraceForObjects _returnvalue (- _returnvalue "0, 0,1.000000") (.Range (Utilities|Struct|BreakTowerStruct (Variables|Default|GetTowerStruct))) (Utilities|Array|MakeArray "ObjectTypeQuery3") false 0 "None"))
  (if _returnvalue_2
    (bind _newtarget (CallFunction|GetClosestTarget _outhits))
    (Utilities|IsValid _newtarget
      (:Is%20Valid
        (Variables|Default|SetCurrentTarget _newtarget))
      (:Is%20Not%20Valid
        _)))
  (Utilities|FlowControl|Delay 0.25)
  (Variables|Default|SetCheckForTarget false))

(event Custom|IncreaseXP
  (params (XPincrease :type Integer))
  (Variables|Default|SetEXP (+ XPincrease (Variables|Default|GetEXP)))
  (CallFunction|CheckLevelUp))

(event Custom|CheckLevelUp
  (if (>= (Variables|Default|GetEXP) (Utilities|Array|Get(acopy) (Variables|Default|GetLevelUp) (+ (Variables|Default|GetCurrentLevel) 1)))
    (bind _result (Math|Integer|IncrementInt (Variables|Default|GetCurrentLevel))
      (:%20%20
        (Development|PrintString (Utilities|String|Append "Tower Level Up! : " (Utilities|String|ToString(Integer) _result)))))))

(event EventBeginPlay
  (bind _returnvalue (Utilities|GetDataTableRow "/Game/Towers/TowerDataTable.TowerDataTable" "AoE")
    (:then
      (Variables|Default|SetTowerStruct _returnvalue)
      (CallFunction|MakeTower))))

(event EventTick
  (params (DeltaSeconds :type Float%20%28single-precision%29))
  (Utilities|IsValid (Variables|Default|GetCurrentTarget)
    (:Is%20Valid
      (if (not (Variables|Default|GetReload))
        (CallFunction|BulletInit)))
    (:Is%20Not%20Valid
      (if (not (Variables|Default|GetCheckForTarget))
        (CallFunction|FindTarget)))))

(fn ConstructionScript)

(fn GetClosestTarget
  (params (HitResults :type Array%20of%20Hit%20Result%20Structures))
  (for _array_element HitResults
    (bind _asenemy (Utilities|Casting|CastToEnemy (.HitActor (Collision|BreakHitResult _array_element))))
    (Utilities|IsValid (LocalVariables|GetTempTarget)
      (:Is%20Valid
        (if (< (Math|Vector|VectorLength (- (Transformation|GetActorLocation) (Transformation|GetActorLocation (.HitActor (Collision|BreakHitResult _array_element))))) (LocalVariables|GetTempDistance))
          (LocalVariables|SetTempTarget _asenemy)
          (LocalVariables|SetTempDistance (Math|Vector|VectorLength (- (Transformation|GetActorLocation) (Transformation|GetActorLocation (.HitActor (Collision|BreakHitResult _array_element))))))))
      (:Is%20Not%20Valid
        (LocalVariables|SetTempTarget _asenemy)
        (LocalVariables|SetTempDistance (Math|Vector|VectorLength (- (Transformation|GetActorLocation) (Transformation|GetActorLocation (.HitActor (Collision|BreakHitResult _array_element)))))))))
  (return (LocalVariables|GetTempTarget)))