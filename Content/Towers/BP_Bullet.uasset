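; Tower projectile that homes on its target enemy and damages it, crediting the owning tower as damage causer.
; Each tick it interpolates toward the target, randomly either playing an explosion sound or adding a fixed diagonal offset, which makes its path jitter.
; It destroys itself when its box overlaps that target or when the target becomes invalid.
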(event OnComponentBeginOverlap(Box)
  (params (OverlappedComponent :type Primitive%20Component%20Object%20Reference) (OtherActor :type Actor%20Object%20Reference) (OtherComp :type Primitive%20Component%20Object%20Reference) (OtherBodyIndex :type Integer) (bFromSweep :type Boolean) (SweepResult :type Hit%20Result%20Structure%20%28by%20ref%29))
  (bind _targetenemy (Variables|Default|GetTargetEnemy))
  (if (== OtherActor _targetenemy)
    (Game|Damage|ApplyDamage _targetenemy (Variables|Default|GetDamage) 0 (Variables|Default|GetTowerOwner))
    (Actor|DestroyActor)))

(event EventTick
  (params (DeltaSeconds :type Float%20%28single-precision%29))
  (bind _returnvalue (Transformation|GetActorLocation))
  (bind _targetenemy (Variables|Default|GetTargetEnemy))
  (bind _bulletspeed (Variables|Default|GetBulletSpeed))
  (bind _returnvalue_2 (Transformation|GetActorLocation _targetenemy))
  (bind _returnvalue_3 (Math|Interpolation|VInterpTo _returnvalue _returnvalue_2 DeltaSeconds _bulletspeed))
  (Utilities|IsValid _targetenemy
    (:Is%20Valid
      (switch int (Math|Random|RandomIntegerinRange 0 1)
        (:0
          (Transformation|SetActorLocation _returnvalue_3 false false)
          (Audio|PlaySound2D "/Game/StarterContent/Audio/Explosion_Cue.Explosion_Cue" 1.0 1.0 0.0 0 0))
        (:1
          (Transformation|SetActorLocation (+ _returnvalue_3 "50.000000,50.000000,50.000000") false false))))
    (:Is%20Not%20Valid
      (Actor|DestroyActor))))

(fn ConstructionScript)